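; BP_Key is an interactable key pickup that sets a key flag on the first-person player character.
; On Interaction it uses IsKey1 to choose which flag to set on BP_FirstPersonCharacter.
; Key 1 also marks its referenced BPDoor as openable and immediately triggers that door's Interaction, while the other key only sets the Key2 flag.
; The key actor then destroys itself.
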(event `/Game/Blueprints/Implemented/BPI_Interaction.Interaction`
  (bind _bp_door (`self.BP_Door`))
  (`|ExecutionSequence`
    (:`then_0`
      (bind _asbp_first_person_character (cast `/Game/Blueprints/Implemented/BP_FirstPersonCharacter` (`GameplayStatics.GetPlayerCharacter` 0)))
      (if (`self.IsKey1`)
        (set `/Game/Blueprints/Implemented/BP_FirstPersonCharacter.Key1` true _asbp_first_person_character)
        (set `/Game/Door_aperture_2_Blueprint.CanOpen` true _bp_door)
        (`/Game/Blueprints/Implemented/BPI_Interaction.Interaction` _bp_door)
        (else
          (set `/Game/Blueprints/Implemented/BP_FirstPersonCharacter.Key2` true _asbp_first_person_character))))
    (:`then_1`
      (`self.K2_DestroyActor`))))

(fn `NewFunction`)

(fn `UserConstructionScript`)